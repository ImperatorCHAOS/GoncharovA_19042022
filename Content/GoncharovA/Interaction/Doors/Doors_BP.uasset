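; Swinging door Blueprint that opens when the MainCharacter enters either of two trigger boxes and closes when they leave.
; Each box plays its own timeline on begin overlap and reverses it on end overlap.
; The timeline track scales Angle for Box1 or AngleReverse for Box2 to set the SMDoor mesh's relative yaw, giving each trigger its own swing angle.
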(event `self.Box1.OnComponentBeginOverlap`
  (params (OverlappedComponent :type "PrimitiveComponent Object Reference") (OtherActor :type "Actor Object Reference") (OtherComp :type "PrimitiveComponent Object Reference") (OtherBodyIndex :type Integer) (bFromSweep :type Boolean) (SweepResult :type "HitResult Structure (by ref)"))
  (cast `/Game/GoncharovA/Characters/MainCharacter` OtherActor)
  (bind (_direction _newtrack_0) (`Timeline|Box 1` :!label _label)
    (:`Update`
      (`SceneComponent.K2_SetRelativeRotation` (`self.SM_Door`) (`KismetMathLibrary.MakeRotator` 0.0 0.0 (* _newtrack_0 (`self.Angle`))) false false))))

(event `self.Box1.OnComponentEndOverlap`
  (params (OverlappedComponent :type "PrimitiveComponent Object Reference") (OtherActor :type "Actor Object Reference") (OtherComp :type "PrimitiveComponent Object Reference") (OtherBodyIndex :type Integer))
  (cast `/Game/GoncharovA/Characters/MainCharacter` OtherActor)
  (goto _label :!via `Reverse`))

(event `self.Box2.OnComponentBeginOverlap`
  (params (OverlappedComponent :type "PrimitiveComponent Object Reference") (OtherActor :type "Actor Object Reference") (OtherComp :type "PrimitiveComponent Object Reference") (OtherBodyIndex :type Integer) (bFromSweep :type Boolean) (SweepResult :type "HitResult Structure (by ref)"))
  (cast `/Game/GoncharovA/Characters/MainCharacter` OtherActor)
  (bind (_direction _newtrack_0) (`Timeline|Box 2` :!label _label_2)
    (:`Update`
      (`SceneComponent.K2_SetRelativeRotation` (`self.SM_Door`) (`KismetMathLibrary.MakeRotator` 0.0 0.0 (* _newtrack_0 (`self.AngleReverse`))) false false))))

(event `self.Box2.OnComponentEndOverlap`
  (params (OverlappedComponent :type "PrimitiveComponent Object Reference") (OtherActor :type "Actor Object Reference") (OtherComp :type "PrimitiveComponent Object Reference") (OtherBodyIndex :type Integer))
  (cast `/Game/GoncharovA/Characters/MainCharacter` OtherActor)
  (goto _label_2 :!via `Reverse`))

(fn `UserConstructionScript`)